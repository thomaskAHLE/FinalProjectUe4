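; BP_StationaryEnemyPawn is an enemy pawn Blueprint, filed with the abstract enemy bases, that adds feedback and player-facing to inherited behavior.
; Being shot spawns a scaled-down blood effect at the hit location and plays a hit sound, while dying plays a death sound.
; Starting an attack rotates it to face the first player's pawn.
; Each of these events then calls its parent implementation.
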(event `self.Die`
  (`GameplayStatics.PlaySoundAtLocation` (`self.DieSound`) (`self.K2_GetActorLocation`) (struct) 1.0 1.0 0.0 null null null)
  (`parent.Die`))

(event `self.OnShot`
  (params (Damage :type "Float (single-precision)") (HitLocation :type "Vector Structure") (ComponentTags :type "Array of Name (by ref)"))
  (`|SpawnActorFromClass` "/Game/FX/Blueprints/BP_ky_hit3_Blood.BP_ky_hit3_Blood_C" (`KismetMathLibrary.MakeTransform` HitLocation (struct) (0.25 0.25 0.25)) "Undefined" "OverrideRootScale" null null)
  (`GameplayStatics.PlaySoundAtLocation` (`self.HitSound`) (`self.K2_GetActorLocation`) (struct) 1.0 1.0 0.0 null null null)
  (`parent.OnShot` Damage HitLocation ComponentTags))

(event `self.StartAttacking`
  (`/Game/Blueprint/EtcBPs/BP_RotateToFaceActor_Func.RotateToFaceActor` self (`GameplayStatics.GetPlayerPawn` 0))
  (`parent.StartAttacking`))

(fn `UserConstructionScript`)