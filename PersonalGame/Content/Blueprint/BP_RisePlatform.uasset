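; BP_RisePlatform is an actor that, once its IsRising flag is set, climbs with a shaking motion and then destroys itself.
; Tick raises Z by a fixed step per frame, so speed depends on frame rate, while X and Y jitter randomly around the position cached at BeginPlay.
; A DoOnce starts the motion through StartTime and a ten-second delay ends it.
; Nothing in this graph sets IsRising to true.
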(event `self.ReceiveBeginPlay`
  (set `self.Location` (`self.K2_GetActorLocation`)))

(event `self.ReceiveTick`
  (params (DeltaSeconds :type "Float (single-precision)"))
  (bind (_returnvalue_x _returnvalue_y _returnvalue_z) (`KismetMathLibrary.BreakVector` (`self.K2_GetActorLocation`)))
  (bind (_location_x _location_y) (`KismetMathLibrary.BreakVector` (`self.Location`)))
  (if (`self.IsRising?`)
    (if (`self.StartTime?`)
      (`self.K2_SetActorLocation` (`KismetMathLibrary.MakeVector` (+ _location_x (`KismetMathLibrary.RandomFloatInRange` -5.0 5.0)) (+ _location_y (`KismetMathLibrary.RandomFloatInRange` -5.0 5.0)) (+ _returnvalue_z 10.0)))
      (else
        (`/Engine/EditorBlueprintResources/StandardMacros.DoOnce` false
          (:`Completed`
            (set `self.StartTime?` true)
            (`KismetSystemLibrary.Delay` 10.0)
            (set `self.IsRising?` false)
            (set `self.StartTime?` false)
            (`self.K2_DestroyActor`)))))))

(fn `UserConstructionScript`)