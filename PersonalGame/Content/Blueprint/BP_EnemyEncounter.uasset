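; BP_EnemyEncounter is a combat encounter that halts the on-rail player until its assigned AI zombies are dead.
; BeginPlay counts the zombies, binds to their death events and holds them still.
; The player's first overlap with StartEnemiesCollision stops the rail pawn and releases the zombies.
; Each death decrements the count; at zero the stored player resumes moving and the encounter destroys itself after a short delay.
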(event `self.ReceiveBeginPlay`
  (bind _aizombies (`self.AIZombies`))
  ;[1 1 1] When the game starts keep all enemies stuck at start position until player overlaps collision.
  (set `self.NumberEnemies` (`KismetArrayLibrary.Array_Length` _aizombies))
  (for _array_element _aizombies
    (`/Engine/EditorBlueprintResources/StandardMacros.IsValid` _array_element
      (:`Is Valid`
        (add `EnemyAICharacter.OnDie` _array_element (delegate `OnEnemyDied`))
        (`EnemyAICharacter.StopMoving` _array_element))
      (:`Is Not Valid`
        (`KismetArrayLibrary.Array_RemoveItem` _aizombies _array_element)))))

(event `OnEnemyDied`
  (bind _overlappedplayer (`self.OverlappedPlayer`))
  (bind _output_get (set `self.NumberEnemies` (- (`self.NumberEnemies`) 1)))
  (`KismetSystemLibrary.PrintString` (`KismetStringLibrary.Conv_IntToString` _output_get) true true (struct :`G` 0.66 :`B` 1.0 :`A` 1.0) -1.0)
  (if (<= _output_get 0)
    (`/Engine/EditorBlueprintResources/StandardMacros.IsValid` _overlappedplayer
      (:`Is Valid`
        (`KismetSystemLibrary.PrintString` "Hello2")
        (`OnRailPawn.StartPawnMoving` _overlappedplayer)
        (`KismetSystemLibrary.Delay` 0.2)
        (`self.K2_DestroyActor`))
      (:`Is Not Valid`
        (`KismetSystemLibrary.PrintString` "Hello")))))

(event `self.StartEnemiesCollision.OnComponentBeginOverlap`
  (params (OverlappedComponent :type "PrimitiveComponent Object Reference") (OtherActor :type "Actor Object Reference") (OtherComp :type "PrimitiveComponent Object Reference") (OtherBodyIndex :type Integer) (bFromSweep :type Boolean) (SweepResult :type "HitResult Structure (by ref)"))
  ;[1 1 1] Start enemies moving towards player. Bind to their onDestroyed function to start player moving when all are killed
  (bind _ason_rail_pawn_player (cast `OnRailPawnPlayer` OtherActor))
  (`/Engine/EditorBlueprintResources/StandardMacros.DoOnce` false
    (:`Completed`
      (bind _output_get (set `self.OverlappedPlayer` _ason_rail_pawn_player))
      (`OnRailPawn.StopPawnMoving` _output_get)
      (for _array_element (`self.AIZombies`)
        (`/Engine/EditorBlueprintResources/StandardMacros.IsValid` _array_element
          (:`Is Valid`
            (`EnemyAICharacter.StartMoving` _array_element)))))))

(fn `UserConstructionScript`)