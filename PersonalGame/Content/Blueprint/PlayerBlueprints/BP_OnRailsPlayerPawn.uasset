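; BP_OnRailsPlayerPawn is the on-rails player pawn, handling input mode, damage feedback and game over.
; BeginPlay sets game-only input, and any damage plays an "Oof" sound at the pawn's location.
; The Die event shows the game-over widget, switches input to UI only and pauses the game.
; The graph contains no movement, health or death-trigger logic.
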(event `self.ReceiveBeginPlay`
  (`WidgetBlueprintLibrary.SetInputMode_GameOnly` (`GameplayStatics.GetPlayerController` 0)))

(event `self.ReceiveAnyDamage`
  (params (Damage :type "Float (single-precision)") (DamageType :type "DamageType Object Reference") (InstigatedBy :type "Controller Object Reference") (DamageCauser :type "Actor Object Reference"))
  (`GameplayStatics.PlaySoundAtLocation` "/Game/FirstPerson/Audio/oof.oof" (`self.K2_GetActorLocation`) (struct) 1.0 1.0 0.0 null null null))

(event `self.Die`
  (bind _returnvalue (`GameplayStatics.GetPlayerController` 0))
  (bind _returnvalue_2 (`|CreateWidget` "/Game/Blueprint/UI_Blueprints/BP_GameOverWidget.BP_GameOverWidget_C" _returnvalue))
  (`UserWidget.AddToViewport` _returnvalue_2 0)
  (`WidgetBlueprintLibrary.SetInputMode_UIOnlyEx` _returnvalue _returnvalue_2)
  (`GameplayStatics.SetGamePaused` true))

(fn `UserConstructionScript`)