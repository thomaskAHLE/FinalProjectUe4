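; BP_ZGuy is a zombie character Blueprint holding action-state and movement logic, none of which runs because no event drives it.
; Hit react, attack, die and spit branches each set a state flag from an Activate boolean and clear Translating while active.
; Translating gates forward and right movement input, whose direction comes from a rotator with control yaw fed into its roll.
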(fn `UserConstructionScript`)