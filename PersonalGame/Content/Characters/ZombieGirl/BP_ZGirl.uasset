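; BP_ZGirl is a player-controlled zombie girl character with movement, death, hit-react and attack inputs.
; Movement axes add input along vectors from a rotator that feeds control yaw into the roll pin, leaving yaw zero.
; Holding an action key sets its state flag and clears Translating to block movement input.
; Releasing any of those keys clears its flag and re-enables movement, even if another is held.
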(event `InputAxis|MoveForward`
  (params (AxisValue :type "Float (single-precision)"))
  (bind (_returnvalue_roll _returnvalue_pitch _returnvalue_yaw) (`KismetMathLibrary.BreakRotator` (`self.GetControlRotation`)))
  ;[1 1 1] Core Movement
  (if (`self.Translating`)
    (`self.AddMovementInput` (`KismetMathLibrary.GetForwardVector` (`KismetMathLibrary.MakeRotator` _returnvalue_yaw)) AxisValue)))

(event `InputAxis|MoveRight`
  (params (AxisValue :type "Float (single-precision)"))
  (bind (_returnvalue_roll _returnvalue_pitch _returnvalue_yaw) (`KismetMathLibrary.BreakRotator` (`self.GetControlRotation`)))
  ;[1 1 1] Core Movement
  (if (`self.Translating`)
    (`self.AddMovementInput` (`KismetMathLibrary.GetRightVector` (`KismetMathLibrary.MakeRotator` _returnvalue_yaw)) AxisValue)))

(event `InputAction|Die`
  (params (Key :type "Key Structure"))
  ;[1 1 1] Die
  (:`Pressed`
    (set `self.IsDying` true)
    (set `self.Translating` false))
  (:`Released`
    (set `self.IsDying` false)
    (set `self.Translating` true)))

(event `InputAction|HitReact`
  (params (Key :type "Key Structure"))
  ;[1 1 1] Hit React
  (:`Pressed`
    (set `self.IsHitReacting` true)
    (set `self.Translating` false))
  (:`Released`
    (set `self.IsHitReacting` false)
    (set `self.Translating` true)))

(event `InputAction|Attack`
  (params (Key :type "Key Structure"))
  ;[1 1 1] Attack
  (:`Pressed`
    (set `self.IsAttacking` true)
    (set `self.Translating` false))
  (:`Released`
    (set `self.IsAttacking` false)
    (set `self.Translating` true)))

(fn `UserConstructionScript`)